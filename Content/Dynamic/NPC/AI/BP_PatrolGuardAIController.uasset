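; AI controller for a patrol guard NPC, driven by a behavior tree and a blackboard.
; On BeginPlay it sets up the PatrolData blackboard and runs the GuardBehaviour tree.
; AI perception updates write any sensed actor without the "Enemy" tag into the blackboard's "Enemy" key.
; A failed sense of such an actor clears that key, without checking which actor it holds.
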(event OnTargetPerceptionUpdated(AIPerception)
  (params (Actor :type Actor%20Object%20Reference) (Stimulus :type AI%20Stimulus%20Structure))
  (if (not (Actor|ActorHasTag Actor "Enemy"))
    (if (.bsuccessfullysensed Stimulus)
      (AI|Components|Blackboard|SetValueasObject (Variables|Default|GetAIBlackboard) (Utilities|Name|MakeLiteralName "Enemy") Actor)
      (else
        (AI|Components|Blackboard|ClearValue (Variables|Default|GetAIBlackboard) (Utilities|Name|MakeLiteralName "Enemy"))))))

(event EventBeginPlay
  (bind _blackboardcomponent (Class|AIController|UseBlackboard "/Game/Dynamic/NPC/AI/PatrolData.PatrolData"))
  (Variables|Default|SetAIBlackboard _blackboardcomponent)
  (AI|RunBehaviorTree "/Game/Dynamic/NPC/AI/GuardBehaviour.GuardBehaviour"))

(event EventTick
  (params (DeltaSeconds :type Float%20%28single-precision%29)))

(fn ConstructionScript)